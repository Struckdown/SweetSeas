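; Selectable cube that the player shoots with a projectile, then sends sliding along the world Y or Z axis.
; A projectile hit deselects all instances, then highlights this one and enables its directional input.
; A direction press locks input, and Tick sweeps it by a frame-rate-dependent step until blocked.
; While moving, a box trace ahead only prints debug messages for possible crushing of the player or other hits.
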(event `self.ReceiveHit`
  (params (MyComp :type "PrimitiveComponent Object Reference") (Other :type "Actor Object Reference") (OtherComp :type "PrimitiveComponent Object Reference") (bSelfMoved :type Boolean) (HitLocation :type "Vector Structure") (HitNormal :type "Vector Structure") (NormalImpulse :type "Vector Structure") (Hit :type "HitResult Structure (by ref)"))
  ;[1 1 1] Deselect previous item
  (cast `/Game/FirstPersonBP/Blueprints/FirstPersonProjectile` Other)
  (bind _outactors (`GameplayStatics.GetAllActorsOfClass` "SelectableObjectZY_C"))
  (bind _output_get (set `self.selectableObjects` _outactors))
  (for _array_element _output_get
    (set `/Game/Blueprints/SelectableObjectZY.selected` false _array_element)
    (set `/Game/Blueprints/SelectableObjectZY.moving` false _array_element)
    (`PrimitiveComponent.SetMaterial` (`/Game/Blueprints/SelectableObjectZY.StaticMesh` _array_element) 0 "/Game/Geometry/Meshes/CubeMaterial.CubeMaterial"))
  (`self.Select Object`))

(event `Select Object`
  ;[1 1 1] Select current object
  (`PrimitiveComponent.SetMaterial` (`self.StaticMesh`) 0 "/Game/StarterContent/Blueprints/Assets/M_LightStage_Skybox_HDRI.M_LightStage_Skybox_HDRI")
  (`self.EnableInput` (`GameplayStatics.GetPlayerController` 0))
  (cast `/Game/FirstPersonBP/Blueprints/FirstPersonCharacter` (`GameplayStatics.GetPlayerCharacter` 0))
  (set `self.selected` true))

(event `InputAction|MoveUp`
  (params (Key :type "Key Structure"))
  ;[1 1 1] Move selected object up
  (:`Pressed`
    (if (`self.selected`)
      (set `self.direction` (0.0 0.0 1.0))
      (`self.Start Move`))))

(event `InputAction|MoveDown`
  (params (Key :type "Key Structure"))
  ;[1 1 1] Move selected object down
  (:`Pressed`
    (if (`self.selected`)
      (set `self.direction` (0.0 0.0 -1.0))
      (`self.Start Move`))))

(event `InputAction|MoveLeft`
  (params (Key :type "Key Structure"))
  ;[1 1 1] Move selected object left
  (:`Pressed`
    (if (`self.selected`)
      (set `self.direction` (0.0 -1.0 0.0))
      (`self.Start Move`))))

(event `InputAction|MoveRight`
  (params (Key :type "Key Structure"))
  ;[1 1 1] Move selected object right
  (:`Pressed`
    (if (`self.selected`)
      (set `self.direction` (0.0 1.0 0.0))
      (`self.Start Move`))))

(event `Start Move`
  ;[1 1 1] Called by MoveUp/Down/Left/Right, sets variable "moving" to true, triggers event tick below
  (`PrimitiveComponent.SetMaterial` (`self.StaticMesh`) 0 "/Game/FirstPerson/Meshes/FirstPersonProjectileMaterial.FirstPersonProjectileMaterial")
  (set `self.selected` false)
  (set `self.moving` true)
  (`self.DisableInput` (`GameplayStatics.GetPlayerController` 0))
  (cast `/Game/FirstPersonBP/Blueprints/FirstPersonCharacter` (`GameplayStatics.GetPlayerCharacter` 0)))

(event `self.ReceiveTick`
  (params (DeltaSeconds :type "Float (single-precision)"))
  (bind _returnvalue (`SceneComponent.K2_GetComponentLocation` (`self.StaticMesh`)))
  (bind _returnvalue_2 (`KismetMathLibrary.MakeTransform` (+ (* (`KismetMathLibrary.Normal` (`self.direction`)) (`self.speed`)) (.location (`SceneComponent.K2_GetComponentToWorld` (`self.StaticMesh`)))) (.rotation (`SceneComponent.K2_GetComponentToWorld` (`self.StaticMesh`))) (.scale (`SceneComponent.K2_GetComponentToWorld` (`self.StaticMesh`)))))
  ;[1 1 1] Moves object on player selected axis (triggered by MoveUp/Down/Left/Right)
  (if (`self.moving`)
    (`self.K2_SetActorTransform` _returnvalue_2 true)
    (if (== _returnvalue_2 (`self.lastPosition`))
      (set `self.moving` false)
      (else
        (set `self.lastPosition` _returnvalue_2)
        ;[1 1 1] Trace in direction cube is travelling for collision
        (if (== (`self.direction`) (0.0 1.0 0.0))
          (`KismetMathLibrary.Vector_Set` (`self.checkCollisionHere`) (.x _returnvalue) (+ (.y _returnvalue) 150.0) (.z _returnvalue))
          (`KismetMathLibrary.Vector_Set` (`self.Half Size`) 30.0 0.0 30.0)
          (bind (_outhits _returnvalue_3) (`KismetSystemLibrary.BoxTraceMultiForObjects` :`Start` _returnvalue :`End` (`self.checkCollisionHere`) :`HalfSize` (`self.Half Size`) :`ObjectTypes` (`self.Object Types`) :`DrawDebugType` "ForDuration" :!label _label))
          (bind _output_get (set `self.Out Hits` _outhits))
          (if _returnvalue_3
            (if (> (`KismetArrayLibrary.Array_Length` _output_get) 1)
              (`KismetSystemLibrary.PrintString` "squish")
              (else
                (bind _asfirst_person_character (cast `/Game/FirstPersonBP/Blueprints/FirstPersonCharacter` (`.HitActor` (`GameplayStatics.BreakHitResult` (`|GetArrayItem` (`self.Out Hits`))))))
                (if true
                  (`KismetSystemLibrary.PrintString` "splat"))))
            (else
              (`KismetSystemLibrary.PrintString` "nope")))
          (elif (== (`self.direction`) (0.0 -1.0 0.0))
            (`KismetMathLibrary.Vector_Set` (`self.checkCollisionHere`) (.x _returnvalue) (+ (.y _returnvalue) -150.0) (.z _returnvalue))
            (`KismetMathLibrary.Vector_Set` (`self.Half Size`) 30.0 0.0 30.0)
            (goto _label)
            (elif (== (`self.direction`) (0.0 0.0 1.0))
              (`KismetMathLibrary.Vector_Set` (`self.checkCollisionHere`) (.x _returnvalue) (.y _returnvalue) (+ (.z _returnvalue) 150.0))
              (`KismetMathLibrary.Vector_Set` (`self.Half Size`) 30.0 30.0)
              (goto _label)
              (elif (== (`self.direction`) (0.0 0.0 -1.0))
                (`KismetMathLibrary.Vector_Set` (`self.checkCollisionHere`) (.x _returnvalue) (.y _returnvalue) (+ (.z _returnvalue) -150.0))
                (`KismetMathLibrary.Vector_Set` (`self.Half Size`) 30.0 30.0)
                (goto _label)))))))))

(fn `UserConstructionScript`)